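; BP_InvisibleWall is a barrier that turns the player back to a fixed point in the level.
; When its Box is hit by a Player-tagged actor, it shows a "No" tutorial message on MainHUD and hides it after a delay.
; It then removes the first-person input mapping context, teleports the actor to a hardcoded location with rotation kept, and restores input shortly after.
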(event `self.Box.OnComponentHit`
  (params (HitComponent :type "PrimitiveComponent Object Reference") (OtherActor :type "Actor Object Reference") (OtherComp :type "PrimitiveComponent Object Reference") (NormalImpulse :type "Vector Structure") (Hit :type "HitResult Structure (by ref)"))
  (bind _returnvalue (pcsubsystem `EnhancedInputLocalPlayerSubsystem` (`GameplayStatics.GetPlayerController` 0)))
  (if (`self.ActorHasTag` OtherActor "Player")
    (bind _asmain_hud (cast `/Game/UI/MainHUD` (`PlayerController.GetHUD` (`GameplayStatics.GetPlayerController` 0))))
    (`/Game/UI/MainHUD.ShowTutorialMessage` _asmain_hud "No")
    (`KismetSystemLibrary.Delay` 3.0)
    (`/Game/UI/MainHUD.HideTutorialMessage` _asmain_hud)
    (`EnhancedInputSubsystemInterface.RemoveMappingContext` _returnvalue "/Game/Input/IMC_FP_Default.IMC_FP_Default" (struct))
    (`KismetSystemLibrary.Delay` 0.2)
    (`self.K2_TeleportTo` OtherActor (4390.0 4100.0 1990.0) (`self.K2_GetActorRotation` OtherActor))
    (`KismetSystemLibrary.Delay` 0.5)
    (`EnhancedInputSubsystemInterface.AddMappingContext` _returnvalue "/Game/Input/IMC_FP_Default.IMC_FP_Default" 0 (struct))))

(fn `UserConstructionScript`)
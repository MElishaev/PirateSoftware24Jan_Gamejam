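; BP_ControlButton is a base actor for a control button that reacts to BP_Bug actors overlapping it, labeled with its ActionType in the construction script.
; Overlap begin counts bugs and enhancing bugs, then calls ModifyAction with the bug's enhancing flag.
; Overlap end calls ClearModification when no bugs remain, but never decrements the enhancing count.
; Both functions are empty stubs here, and the player character is cached at BeginPlay.
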(event `self.ReceiveBeginPlay`
  (bind _asbp_first_person_character (cast `/Game/FirstPerson/Blueprints/BP_FirstPersonCharacter` (`GameplayStatics.GetPlayerPawn` 0)))
  (set `self.PlayerCharacter` _asbp_first_person_character))

(event `self.ButtonOverlap.OnComponentBeginOverlap`
  (params (OverlappedComponent :type "PrimitiveComponent Object Reference") (OtherActor :type "Actor Object Reference") (OtherComp :type "PrimitiveComponent Object Reference") (OtherBodyIndex :type Integer) (bFromSweep :type Boolean) (SweepResult :type "HitResult Structure (by ref)"))
  (if (`KismetMathLibrary.ClassIsChildOf` (`GameplayStatics.GetObjectClass` OtherActor) "/Game/Blueprints/Bugs/BP_Bug.BP_Bug_C")
    (`/Engine/EditorBlueprintResources/StandardMacros.IncrementInt` (`self.NumOverlappingBugs`)
      (:`  `
        (bind _asbp_bug (cast `/Game/Blueprints/Bugs/BP_Bug` OtherActor))
        (bind _isenhancingbug (`/Game/Blueprints/Bugs/BP_Bug.IsEnhancingBug` _asbp_bug))
        (if _isenhancingbug
          (`/Engine/EditorBlueprintResources/StandardMacros.IncrementInt` (`self.NumEnhancingBugs`)
            (:`  `
              _)))
        (`self.ModifyAction` _isenhancingbug)))))

(event `self.ButtonOverlap.OnComponentEndOverlap`
  (params (OverlappedComponent :type "PrimitiveComponent Object Reference") (OtherActor :type "Actor Object Reference") (OtherComp :type "PrimitiveComponent Object Reference") (OtherBodyIndex :type Integer))
  (if (`KismetMathLibrary.ClassIsChildOf` (`GameplayStatics.GetObjectClass` OtherActor) "/Game/Blueprints/Bugs/BP_Bug.BP_Bug_C")
    (`/Engine/EditorBlueprintResources/StandardMacros.DecrementInt` (`self.NumOverlappingBugs`)
      (:`  `
        (if (== (`self.NumOverlappingBugs`) 0)
          (`self.ClearModification`))))))

(fn `ClearModification`)

(fn `ModifyAction`
  (params (IsEnhance :type Boolean)))

(fn `UserConstructionScript`
  (`TextRenderComponent.K2_SetText` (`self.TextRender`) (`KismetTextLibrary.Conv_StringToText` (`|GetEnumeratorNameAsString` (`self.ActionType`)))))